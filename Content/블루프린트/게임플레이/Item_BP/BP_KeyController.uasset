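; Controller actor that spawns BP_Key pickups at random BP_KeySpawnLoc points, gated by a "ghost caught" flag (유령이잡혔을때).
; BeginPlay caches the spawn point transforms and clears the flag, which nothing in this file initially sets to true.
; Tick calls 열쇠소환, which consumes the flag and spawns a key if fewer than two exist.
; After spawning, it re-arms the flag if Gameplay_GM's IsCaptured equals 0.
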(event `self.ReceiveBeginPlay`
  ;[1 1 1] 시작할때 위치 파악
  (bind _outactors (`GameplayStatics.GetAllActorsOfClass` "/Game/블루프린트/게임플레이/Item_BP/BP_KeySpawnLoc.BP_KeySpawnLoc_C"))
  (for _array_element _outactors
    (`KismetArrayLibrary.Array_Add` (`self.transformSpots`) (`self.GetTransform` _array_element))
    (set `self.유령이 잡혔을 때` false)))

(event `열쇠소환`
  ;[1 1 1] 맵에 하나 열쇠 소환
  (if (`self.유령이 잡혔을 때`)
    (set `self.유령이 잡혔을 때` false)
    (bind _outactors (`GameplayStatics.GetAllActorsOfClass` "/Game/블루프린트/게임플레이/Item_BP/BP_Key.BP_Key_C"))
    (if (< (`KismetArrayLibrary.Array_Length` _outactors) 2)
      (`|SpawnActorFromClass` "/Game/블루프린트/게임플레이/Item_BP/BP_Key.BP_Key_C" (`KismetArrayLibrary.Array_Get` (`self.transformSpots`) (`KismetMathLibrary.RandomInteger` (`KismetArrayLibrary.Array_Length` (`self.transformSpots`)))) "Undefined" "OverrideRootScale")
      (bind _asgameplay_gm (cast `/Game/블루프린트/게임플레이/GamePlay/Gameplay_GM` (`GameplayStatics.GetGameMode`)))
      (if (== (`/Game/블루프린트/게임플레이/GamePlay/Gameplay_GM.IsCaptured` _asgameplay_gm) 0)
        (set `self.유령이 잡혔을 때` true)))))

(event `self.ReceiveTick`
  (params (DeltaSeconds :type "Float (single-precision)"))
  ;[1 1 1] 맵에 하나 열쇠 소환
  (`self.열쇠소환`))

(fn `OnRep_test`)

(fn `UserConstructionScript`)