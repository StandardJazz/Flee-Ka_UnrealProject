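; BP_CostController respawns the BP_Cost items in the level once all of them are gone.
; On BeginPlay it caches the transform of every BP_CostSpawnLoc actor in FirstLocation.
; Tick polls the IsDestroyed flag, clears it, and checks whether any BP_Cost actors remain.
; If none remain, it waits through a fixed delay, then spawns a new BP_Cost at each cached transform.
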(event `self.ReceiveBeginPlay`
  ;[1 1 1] 처음 위치 transform배열로 만들기
  (bind _outactors (`GameplayStatics.GetAllActorsOfClass` "/Game/블루프린트/게임플레이/Item_BP/BP_CostSpawnLoc.BP_CostSpawnLoc_C"))
  (for _array_element _outactors
    (`KismetArrayLibrary.Array_Add` (`self.FirstLocation`) (`self.GetTransform` _array_element))))

(event `self.ReceiveTick`
  (params (DeltaSeconds :type "Float (single-precision)"))
  ;[1 1 1] 코스트 다먹으면 일정 카운트 뒤에 다시 생성
  (if (`self.isDestroyed`)
    (set `self.isDestroyed` false)
    (bind _outactors (`GameplayStatics.GetAllActorsOfClass` "/Game/블루프린트/게임플레이/Item_BP/BP_Cost.BP_Cost_C"))
    (if (<= (`KismetArrayLibrary.Array_Length` _outactors) 0)
      (`KismetSystemLibrary.Delay` 10.0)
      (for _array_element (`self.FirstLocation`)
        (`|SpawnActorFromClass` "/Game/블루프린트/게임플레이/Item_BP/BP_Cost.BP_Cost_C" _array_element "Undefined" "OverrideRootScale")))))

(fn `UserConstructionScript`)