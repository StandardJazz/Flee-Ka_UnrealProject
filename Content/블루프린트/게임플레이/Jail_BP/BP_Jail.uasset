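; BP_Jail is a jail actor that registers a captured demon (ghost) when one overlaps its DemonTrigger component.
; The overlap calls a custom event that casts the actor to the base demon class and passes through a DoOnce.
; It then increments IsCaptured on Gameplay_GM and clears the demon's three key flags.
; The DoOnce has no reset here, so each jail instance counts only one capture.
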(event `self.DemonTrigger.OnComponentBeginOverlap`
  (params (OverlappedComponent :type "PrimitiveComponent Object Reference") (OtherActor :type "Actor Object Reference") (OtherComp :type "PrimitiveComponent Object Reference") (OtherBodyIndex :type Integer) (bFromSweep :type Boolean) (SweepResult :type "HitResult Structure (by ref)"))
  ;[1 1 1] 유령카운트
  (`self.감옥안에 유령카운트` OtherActor))

(event `감옥안에 유령카운트`
  (params (Target :type "Actor Object Reference"))
  ;[1 1 1] 유령카운트
  (bind `_asdemon_bp_0기본` (cast `/Game/블루프린트/캐릭터/엑터/DemonBP_0기본` Target))
  (`/Engine/EditorBlueprintResources/StandardMacros.DoOnce` false
    (:`Completed`
      (bind _asgameplay_gm (cast `/Game/블루프린트/게임플레이/GamePlay/Gameplay_GM` (`GameplayStatics.GetGameMode`)))
      (set `/Game/블루프린트/게임플레이/GamePlay/Gameplay_GM.IsCaptured` (+ (`/Game/블루프린트/게임플레이/GamePlay/Gameplay_GM.IsCaptured` _asgameplay_gm) 1) _asgameplay_gm)
      (set `/Game/블루프린트/캐릭터/엑터/DemonBP_0기본.HaveKey1` false `_asdemon_bp_0기본`)
      (set `/Game/블루프린트/캐릭터/엑터/DemonBP_0기본.HaveKey2` false `_asdemon_bp_0기본`)
      (set `/Game/블루프린트/캐릭터/엑터/DemonBP_0기본.HaveKey3` false `_asdemon_bp_0기본`))))

(fn `UserConstructionScript`)