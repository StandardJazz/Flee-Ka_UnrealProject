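; BP_OpenPoint is a trigger point that lets a key-carrying demon character open the jail for a jailbreak.
; Overlapping KeyTrigger calls the 감옥탈출 (jail escape) event, which checks whether the DemonBP_0기본 actor holds any of three keys.
; It destroys the first BP_Jail found, respawns one at a hardcoded location after a delay, then resets Gameplay_GM's IsCaptured and clears that character's keys.
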(event `self.KeyTrigger.OnComponentBeginOverlap`
  (params (OverlappedComponent :type "PrimitiveComponent Object Reference") (OtherActor :type "Actor Object Reference") (OtherComp :type "PrimitiveComponent Object Reference") (OtherBodyIndex :type Integer) (bFromSweep :type Boolean) (SweepResult :type "HitResult Structure (by ref)"))
  ;[1 1 1] 감옥탈출시키기
  (`self.감옥탈출` OtherActor))

(event `감옥탈출`
  (params (OtherActor :type "Actor Object Reference"))
  ;[1 1 1] 감옥탈출시키기
  (bind _outactors (`GameplayStatics.GetAllActorsOfClass` "/Game/블루프린트/게임플레이/Jail_BP/BP_Jail.BP_Jail_C"))
  (bind `_asdemon_bp_0기본` (cast `/Game/블루프린트/캐릭터/엑터/DemonBP_0기본` OtherActor))
  (if (or (`/Game/블루프린트/캐릭터/엑터/DemonBP_0기본.HaveKey1` `_asdemon_bp_0기본`) (`/Game/블루프린트/캐릭터/엑터/DemonBP_0기본.HaveKey2` `_asdemon_bp_0기본`) (`/Game/블루프린트/캐릭터/엑터/DemonBP_0기본.HaveKey3` `_asdemon_bp_0기본`))
    (`self.K2_DestroyActor` (`KismetArrayLibrary.Array_Get` _outactors))
    (`KismetSystemLibrary.Delay` 2.0)
    (`|SpawnActorFromClass` "/Game/블루프린트/게임플레이/Jail_BP/BP_Jail.BP_Jail_C" (`KismetMathLibrary.MakeTransform` (-430.0 2600.0 6400.0)) "Undefined" "OverrideRootScale")
    (bind _asgameplay_gm (cast `/Game/블루프린트/게임플레이/GamePlay/Gameplay_GM` (`GameplayStatics.GetGameMode`)))
    (set `/Game/블루프린트/게임플레이/GamePlay/Gameplay_GM.IsCaptured` 0 _asgameplay_gm)
    (set `/Game/블루프린트/캐릭터/엑터/DemonBP_0기본.HaveKey1` false `_asdemon_bp_0기본`)
    (set `/Game/블루프린트/캐릭터/엑터/DemonBP_0기본.HaveKey2` false `_asdemon_bp_0기본`)
    (set `/Game/블루프린트/캐릭터/엑터/DemonBP_0기본.HaveKey3` false `_asdemon_bp_0기본`)))

(fn `UserConstructionScript`)